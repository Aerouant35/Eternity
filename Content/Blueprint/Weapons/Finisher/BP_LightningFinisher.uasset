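; BP_LightningFinisher is a lightning finisher attack for the transcendent form, launched through LaunchFinisher.
; It disables the owning character's input and activates a Niagara effect placed ahead of them, facing their rotation.
; A looping timer box-traces that area to damage each BP_Enemy hit.
; After FinisherDuration, it clears the timer, deactivates the effect and transcendent form, and restores input.
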(event Custom|LightningHit
  (bind _transcendent_form_component (Variables|Default|GetTranscendent%20Form%20Component))
  (bind _returnvalue (Components|GetOwner _transcendent_form_component))
  (bind _pos (CallFunction|SetPos))
  (bind _outhits (Class|KismetSystemLibrary|BoxTraceMulti _pos _pos "500.000000,500.000000,200.000000" (Transformation|GetActorRotation _returnvalue) "TraceTypeQuery1" false (Utilities|Array|MakeArray _returnvalue) "None" true))
  (for _array_element _outhits
    (bind _asbp_enemy (Utilities|Casting|CastToBP_Enemy (.HitActor (Collision|BreakHitResult _array_element))))
    (Class|HealthComponent|TakeDamage (Variables|/Game/Blueprint/Ennemies/BP_Enemy.BP_Enemy_C|GetHealth _asbp_enemy) (Utilities|Struct|MakeHitInfo 1))))

(event EventBeginPlay)

(event Collision|EventActorBeginOverlap
  (params (OtherActor :type Actor%20Object%20Reference)))

(event EventTick
  (params (DeltaSeconds :type Float%20%28single-precision%29)))

(event EventLaunchFinisher
  (params (TranscendentFormComponent :type Transcendent%20Form%20Component%20Object%20Reference))
  (bind _niagara (Variables|Default|GetNiagara))
  (Variables|Default|SetTranscendent%20Form%20Component TranscendentFormComponent)
  (bind _returnvalue (Utilities|Time|SetTimerbyEvent (delegate Custom|LightningHit) (Variables|Default|GetDamagePerSec) true))
  (CallFunction|EnablePlayer false)
  (Components|Activation|Activate _niagara false)
  (Transformation|SetWorldRotation _niagara (Transformation|GetActorRotation (Components|GetOwner (Variables|Default|GetTranscendent%20Form%20Component))) false false)
  (bind _pos (CallFunction|SetPos))
  (Transformation|SetWorldLocation (Variables|Default|GetNiagara) _pos false false)
  (Utilities|FlowControl|Delay (Variables|Default|GetFinisherDuration))
  (Utilities|Time|ClearandInvalidateTimerbyHandle _returnvalue)
  (Variables|/Script/Eternity.TranscendentFormComponent|SetbIsFinisherActive (Variables|Default|GetTranscendent%20Form%20Component) false)
  (Class|TranscendentFormComponent|DeactivateTranscendentForm (Variables|Default|GetTranscendent%20Form%20Component))
  (Components|Activation|Deactivate (Variables|Default|GetNiagara))
  (CallFunction|EnablePlayer true))

(fn ConstructionScript)

(fn SetPos
  (bind _transcendent_form_component (Variables|Default|GetTranscendent%20Form%20Component))
  (bind _returnvalue (Components|GetOwner _transcendent_form_component))
  (return (+ (Transformation|GetActorLocation _returnvalue) (* (Transformation|GetActorForwardVector _returnvalue) (Variables|Default|GetSizeDelta)))))

(fn EnablePlayer
  (params (Enable :type Boolean))
  (bind _aseternity_character (Utilities|Casting|CastToEternityCharacter (Components|GetOwner (Variables|Default|GetTranscendent%20Form%20Component))))
  (Class|EternityCharacter|EnableEnhancedInput _aseternity_character Enable))