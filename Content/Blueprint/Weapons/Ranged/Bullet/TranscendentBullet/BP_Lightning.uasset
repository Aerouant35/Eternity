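; BP_Lightning is a lightning bullet that deals area damage around the enemy it strikes.
; On overlapping a BP_Enemy, it runs a zero-length multi sphere trace on the Visibility channel at that enemy, with persistent debug drawing left on.
; Enemies found by the trace and the struck enemy take the base damage through their Health.
; The bullet then destroys itself, as it does when overlapping any other actor.
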(event EventBeginPlay)

(event Collision|EventActorBeginOverlap
  (params (OtherActor :type Actor%20Object%20Reference))
  (bind _asbp_enemy (Utilities|Casting|CastToBP_Enemy OtherActor)
    (:then
      (bind _outhits (Collision|MultiSphereTraceByChannel (Transformation|GetActorLocation _asbp_enemy) (Transformation|GetActorLocation _asbp_enemy) (Variables|Default|GetSphereRadius) "TraceTypeQuery1" false (Utilities|Array|MakeArray _asbp_enemy) "Persistent"))
      (for _array_element _outhits
        (bind _asbp_enemy_2 (Utilities|Casting|CastToBP_Enemy (.HitActor (Collision|BreakHitResult _array_element))))
        (Class|HealthComponent|TakeDamage (Variables|/Game/Blueprint/Ennemies/BP_Enemy.BP_Enemy_C|GetHealth _asbp_enemy_2) (Utilities|Struct|MakeHitInfo (Math|Float|Truncate (Variables|Default|GetBaseDamage)))))
      (Class|HealthComponent|TakeDamage (Variables|/Game/Blueprint/Ennemies/BP_Enemy.BP_Enemy_C|GetHealth _asbp_enemy) (Utilities|Struct|MakeHitInfo (Math|Float|Truncate (Variables|Default|GetBaseDamage))))
      (Actor|DestroyActor))
    (:CastFailed
      (Actor|DestroyActor))))

(event EventTick
  (params (DeltaSeconds :type Float%20%28single-precision%29)))

(fn ConstructionScript)